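; BP_MasterItem is a pickup item actor, apparently a base class, carrying an ItemInfo struct for display, document, stat and equipment data.
; Its sphere overlaps increment and decrement TimerOverlap on the player's BP_VystudioCharacterController character.
; ActionOn enables pickup, custom-depth highlight and the widget, then a short retriggerable delay clears them unless it is called again.
; DestroySphere and EnableSphere toggle the sphere's Pawn collision response, with DestroySphere also hiding highlight and widget.
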(event `self.ReceiveBeginPlay`
  (bind _asbp_vystudio_character_controller (cast `/Game/TPSProPack/Controllers/CharBlueprints/BP_VystudioCharacterController` (`GameplayStatics.GetPlayerCharacter` 0)))
  (set `self.VSRef` _asbp_vystudio_character_controller))

(event `self.Sphere.OnComponentBeginOverlap`
  (params (OverlappedComponent :type "PrimitiveComponent Object Reference") (OtherActor :type "Actor Object Reference") (OtherComp :type "PrimitiveComponent Object Reference") (OtherBodyIndex :type Integer) (bFromSweep :type Boolean) (SweepResult :type "HitResult Structure (by ref)"))
  (bind _vsref (`self.VSRef`))
  (set `/Game/TPSProPack/Controllers/CharBlueprints/BP_VystudioCharacterController.TimerOverlap` (+ (`/Game/TPSProPack/Controllers/CharBlueprints/BP_VystudioCharacterController.TimerOverlap` _vsref) 1.0) _vsref))

(event `self.Sphere.OnComponentEndOverlap`
  (params (OverlappedComponent :type "PrimitiveComponent Object Reference") (OtherActor :type "Actor Object Reference") (OtherComp :type "PrimitiveComponent Object Reference") (OtherBodyIndex :type Integer))
  (bind _vsref (`self.VSRef`))
  (set `/Game/TPSProPack/Controllers/CharBlueprints/BP_VystudioCharacterController.TimerOverlap` (- (`/Game/TPSProPack/Controllers/CharBlueprints/BP_VystudioCharacterController.TimerOverlap` _vsref) 1.0) _vsref))

(event `ActionOn`
  (set `/Game/TPSProPack/Controllers/CharBlueprints/BP_VystudioCharacterController.CanWePickup` true (`self.VSRef`))
  (`PrimitiveComponent.SetRenderCustomDepth` (`self.StaticMesh`) true)
  (`SceneComponent.SetVisibility` (`self.Widget`) true false)
  (set `self.Timer` 0.1)
  (`KismetSystemLibrary.RetriggerableDelay` (`self.Timer`))
  (set `/Game/TPSProPack/Controllers/CharBlueprints/BP_VystudioCharacterController.CanWePickup` false (`self.VSRef`))
  (`self.ActionOff`))

(event `ActionOff`
  (`PrimitiveComponent.SetRenderCustomDepth` (`self.StaticMesh`) false)
  (`SceneComponent.SetVisibility` (`self.Widget`) false false))

(event `DestroySphere`
  (`PrimitiveComponent.SetRenderCustomDepth` (`self.StaticMesh`) false)
  (`PrimitiveComponent.SetCollisionResponseToChannel` (`self.Sphere`) "ECC_Pawn" "ECR_Ignore")
  (`SceneComponent.SetVisibility` (`self.Widget`) false false))

(event `EnableSphere`
  (`PrimitiveComponent.SetCollisionResponseToChannel` (`self.Sphere`) "ECC_Pawn" "ECR_Overlap"))

(fn `UserConstructionScript`
  (bind (_iteminfo_name _iteminfo_image _iteminfo_description _iteminfo_weight _iteminfo_documenttitle _iteminfo_documenttext _iteminfo_documentpictures _iteminfo_addhealth _iteminfo_addenergy _iteminfo_equipsocket _iteminfo_armortypeonlyforarmor) (break `/Game/TPSProPack/Controllers/BPObjects/Item/InventoryItem_Structure` (`self.ItemInfo`)))
  (set `self.ItemInfo` (make `/Game/TPSProPack/Controllers/BPObjects/Item/InventoryItem_Structure` _iteminfo_name _iteminfo_image _iteminfo_description _iteminfo_weight _iteminfo_documenttitle _iteminfo_documenttext _iteminfo_documentpictures _iteminfo_addhealth _iteminfo_addenergy _iteminfo_equipsocket _iteminfo_armortypeonlyforarmor)))