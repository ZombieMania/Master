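; Master elevator Blueprint that carries a platform mesh between seven preset floor heights chosen through a UI widget.
; Interaction events briefly outline the button mesh and flag it usable on the Vystudio character, then open the widget in UI-only input.
; Tick polls the widget's selected floor and moves the platform at constant speed using FInterpToConstant.
; A box trigger adjusts the character's TimerOverlap counter on enter and exit.
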(event `self.ReceiveBeginPlay`
  (bind _asbp_vystudio_character_controller (cast `/Game/TPSProPack/Controllers/CharBlueprints/BP_VystudioCharacterController` (`GameplayStatics.GetPlayerCharacter` 0)))
  (set `self.VSRef` _asbp_vystudio_character_controller)
  (bind _returnvalue (`|CreateWidget` "/Game/TPSProPack/Controllers/BPObjects/Elevator/ElevatorWidget.ElevatorWidget_C"))
  (set `self.WidjetButton` _returnvalue)
  (set `self.CurrentLocation` (0.0 0.0 0.0))
  (set `self.CurrentPos` 1))

(event `self.ReceiveTick`
  (params (DeltaSeconds :type "Float (single-precision)"))
  (if (== (`/Game/TPSProPack/Controllers/BPObjects/Elevator/ElevatorWidget.Pos` (`self.WidjetButton`)) 0)
    (set `self.ToLocation` (0.0 0.0 0.0))
    (elif (== (`/Game/TPSProPack/Controllers/BPObjects/Elevator/ElevatorWidget.Pos` (`self.WidjetButton`)) 1)
      (set `self.ToLocation` (0.0 0.0 0.0))
      (set `self.CurrentPos` 1)
      (`self.1`)
      (elif (== (`/Game/TPSProPack/Controllers/BPObjects/Elevator/ElevatorWidget.Pos` (`self.WidjetButton`)) 2)
        (set `self.ToLocation` (0.0 0.0 450.0))
        (set `self.CurrentPos` 2)
        (`self.2`)
        (elif (== (`/Game/TPSProPack/Controllers/BPObjects/Elevator/ElevatorWidget.Pos` (`self.WidjetButton`)) 3)
          (set `self.ToLocation` (0.0 0.0 960.0))
          (set `self.CurrentPos` 3)
          (`self.3`)
          (elif (== (`/Game/TPSProPack/Controllers/BPObjects/Elevator/ElevatorWidget.Pos` (`self.WidjetButton`)) 4)
            (set `self.ToLocation` (0.0 0.0 1400.0))
            (set `self.CurrentPos` 4)
            (`self.4`)
            (elif (== (`/Game/TPSProPack/Controllers/BPObjects/Elevator/ElevatorWidget.Pos` (`self.WidjetButton`)) 5)
              (set `self.ToLocation` (0.0 0.0 1900.0))
              (set `self.CurrentPos` 5)
              (`self.5`)
              (elif (== (`/Game/TPSProPack/Controllers/BPObjects/Elevator/ElevatorWidget.Pos` (`self.WidjetButton`)) 6)
                (set `self.ToLocation` (0.0 0.0 2400.0))
                (set `self.CurrentPos` 6)
                (`self.6`)
                (elif (== (`/Game/TPSProPack/Controllers/BPObjects/Elevator/ElevatorWidget.Pos` (`self.WidjetButton`)) 7)
                  (set `self.ToLocation` (0.0 0.0 2850.0))
                  (set `self.CurrentPos` 7)
                  (`self.7`))))))))))

(event `self.Box.OnComponentBeginOverlap`
  (params (OverlappedComponent :type "PrimitiveComponent Object Reference") (OtherActor :type "Actor Object Reference") (OtherComp :type "PrimitiveComponent Object Reference") (OtherBodyIndex :type Integer) (bFromSweep :type Boolean) (SweepResult :type "HitResult Structure (by ref)"))
  (set `/Game/TPSProPack/Controllers/CharBlueprints/BP_VystudioCharacterController.TimerOverlap` (+ (`/Game/TPSProPack/Controllers/CharBlueprints/BP_VystudioCharacterController.TimerOverlap` (`self.VSRef`)) 1.0) (`self.VSRef`)))

(event `self.Box.OnComponentEndOverlap`
  (params (OverlappedComponent :type "PrimitiveComponent Object Reference") (OtherActor :type "Actor Object Reference") (OtherComp :type "PrimitiveComponent Object Reference") (OtherBodyIndex :type Integer))
  (set `/Game/TPSProPack/Controllers/CharBlueprints/BP_VystudioCharacterController.TimerOverlap` (- (`/Game/TPSProPack/Controllers/CharBlueprints/BP_VystudioCharacterController.TimerOverlap` (`self.VSRef`)) 1.0) (`self.VSRef`)))

(event `ActionOn`
  (params (NewParam :type "ActorComponent Object Reference"))
  (if (== NewParam (`self.StaticMesh1`))
    (set `/Game/TPSProPack/Controllers/CharBlueprints/BP_VystudioCharacterController.CanWePickup` true (`self.VSRef`))
    (`PrimitiveComponent.SetRenderCustomDepth` (`self.StaticMesh1`) true)
    (set `self.Timer` 0.1)
    (`KismetSystemLibrary.RetriggerableDelay` (`self.Timer`))
    (set `/Game/TPSProPack/Controllers/CharBlueprints/BP_VystudioCharacterController.CanWePickup` false (`self.VSRef`))
    (`PrimitiveComponent.SetRenderCustomDepth` (`self.StaticMesh1`) false)))

(event `Action`
  (bind _returnvalue (`GameplayStatics.GetPlayerController` 0))
  (`UserWidget.AddToViewport` (`self.WidjetButton`) 0)
  (set `PlayerController.bShowMouseCursor` true _returnvalue)
  (`WidgetBlueprintLibrary.SetInputMode_UIOnlyEx` _returnvalue null))

(event `1`
  (bind (_currentlocation_x _currentlocation_y _currentlocation_z) (`KismetMathLibrary.BreakVector` (`self.CurrentLocation`)))
  (bind (_tolocation_x _tolocation_y _tolocation_z) (`KismetMathLibrary.BreakVector` (`self.ToLocation`)))
  (bind _returnvalue (`KismetMathLibrary.MakeVector` 0.0 0.0 (`KismetMathLibrary.FInterpTo_Constant` _currentlocation_z _tolocation_z (`GameplayStatics.GetWorldDeltaSeconds`) 200.0)))
  (if (not (== (`self.CurrentLocation`) (`self.ToLocation`) :`ErrorTolerance` 1.0)) :!label _label
    (`SceneComponent.K2_SetRelativeLocation` (`self.StaticMesh`) _returnvalue false false)
    (set `self.CurrentLocation` _returnvalue)))

(event `2`
  (goto _label))

(event `3`
  (goto _label))

(event `4`
  (goto _label))

(event `5`
  (goto _label))

(event `6`
  (goto _label))

(event `7`
  (goto _label))

(fn `UserConstructionScript`)