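; Card detector base actor that sets a timed door-open status when the player's inventory holds the required card class.
; Box overlaps adjust the character's overlap counter; ActionOn briefly enables pickup and a custom-depth highlight through a retriggerable delay.
; Open switches green/red LEDs on all detectors of the same class, or briefly shows a find-card widget if the card is missing.
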(event `self.ReceiveBeginPlay`
  (bind _asbp_vystudio_character_controller (cast `/Game/TPSProPack/Controllers/CharBlueprints/BP_VystudioCharacterController` (`GameplayStatics.GetPlayerCharacter` 0)))
  (set `self.VSRef` _asbp_vystudio_character_controller)
  (bind _outactors (`GameplayStatics.GetAllActorsOfClass` (`GameplayStatics.GetObjectClass` self)))
  (bind _output_get (set `self.ActorsOfClass` _outactors))
  (`self.LED_Off` _output_get))

(event `self.Box.OnComponentBeginOverlap`
  (params (OverlappedComponent :type "PrimitiveComponent Object Reference") (OtherActor :type "Actor Object Reference") (OtherComp :type "PrimitiveComponent Object Reference") (OtherBodyIndex :type Integer) (bFromSweep :type Boolean) (SweepResult :type "HitResult Structure (by ref)"))
  (bind _vsref (`self.VSRef`))
  (set `/Game/TPSProPack/Controllers/CharBlueprints/BP_VystudioCharacterController.TimerOverlap` (+ (`/Game/TPSProPack/Controllers/CharBlueprints/BP_VystudioCharacterController.TimerOverlap` _vsref) 1.0) _vsref))

(event `self.Box.OnComponentEndOverlap`
  (params (OverlappedComponent :type "PrimitiveComponent Object Reference") (OtherActor :type "Actor Object Reference") (OtherComp :type "PrimitiveComponent Object Reference") (OtherBodyIndex :type Integer))
  (bind _vsref (`self.VSRef`))
  (set `/Game/TPSProPack/Controllers/CharBlueprints/BP_VystudioCharacterController.TimerOverlap` (- (`/Game/TPSProPack/Controllers/CharBlueprints/BP_VystudioCharacterController.TimerOverlap` _vsref) 1.0) _vsref))

(event `ActionOn`
  (set `/Game/TPSProPack/Controllers/CharBlueprints/BP_VystudioCharacterController.CanWePickup` true (`self.VSRef`))
  (`PrimitiveComponent.SetRenderCustomDepth` (`self.StaticMesh`) true)
  (set `self.Timer` 0.1)
  (`KismetSystemLibrary.RetriggerableDelay` (`self.Timer`))
  (set `/Game/TPSProPack/Controllers/CharBlueprints/BP_VystudioCharacterController.CanWePickup` false (`self.VSRef`))
  (`self.ActionOff`))

(event `ActionOff`
  (`PrimitiveComponent.SetRenderCustomDepth` (`self.StaticMesh`) false))

(event `Open`
  (bind _actorsofclass (`self.ActorsOfClass`))
  ;[1 1 1] Open door status
  (if (`KismetArrayLibrary.Array_Contains` (`.AllItemsClass_20_540E31F4492AFE481071AABAD10270D5` (break `/Game/TPSProPack/Controllers/CharBlueprints/Structure/BP_ItemStructure` (`/Game/TPSProPack/Controllers/CharBlueprints/BP_VystudioCharacterController.ItemArray` (`self.VSRef`)))) (`self.Card`))
    (set `self.OpenStatus` true)
    (`self.LED_On` _actorsofclass)
    (`KismetSystemLibrary.RetriggerableDelay` 5.0)
    (set `self.OpenStatus` false)
    (`self.LED_Off` _actorsofclass)
    (else
      (set `self.OpenStatus` false)
      (`self.LED_Off` _actorsofclass)
      (`|ExecutionSequence`
        (:`then_0`
          (`/Engine/EditorBlueprintResources/StandardMacros.DoOnce` false
            (:`Completed`
              (bind _returnvalue (`|CreateWidget` "/Game/TPSProPack/Controllers/Interface/UI/BP_FindCardUI.BP_FindCardUI_C"))
              (set `self.FindCardUI` _returnvalue))))
        (:`then_1`
          (`/Engine/EditorBlueprintResources/StandardMacros.DoOnce` false :!label _label
            (:`Completed`
              (`UserWidget.AddToViewport` (`self.FindCardUI`) 0)
              (`KismetSystemLibrary.RetriggerableDelay` 2.0)
              (`Widget.RemoveFromParent` (`self.FindCardUI`))
              (goto _label :!via `Reset`))))))))

(event `LED_On`
  ;[1 1 1] Open
  (`LightComponent.SetIntensity` (`self.Green`) 100.0)
  (`LightComponent.SetIntensity` (`self.Red`) 0.0))

(event `LED_Off`
  ;[1 1 1] Close
  (`LightComponent.SetIntensity` (`self.Green`) 0.0)
  (`LightComponent.SetIntensity` (`self.Red`) 100.0))

(fn `UserConstructionScript`)