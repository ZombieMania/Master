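; Master door Blueprint that swings open and closed on a timeline, locked by key, card or code according to DoorCategory.
; Key doors check the player's inventory, unlock before a later Open swings them, or show a find-key widget.
; Card and code doors poll the first detectors returned by GetAllActorsOfClass rather than linked references.
; Box overlaps adjust the character's overlap counter, while ActionOn briefly enables pickup and custom-depth highlighting.
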(event `self.ReceiveBeginPlay`
  (bind _asbp_vystudio_character_controller (cast `/Game/TPSProPack/Controllers/CharBlueprints/BP_VystudioCharacterController` (`GameplayStatics.GetPlayerCharacter` 0)))
  (set `self.VSRef` _asbp_vystudio_character_controller)
  (bind _returnvalue (`GameplayStatics.CreateSound2D` (`self.Open/CloseDoorSound`) 1.0 1.0 0.0 null false false))
  (set `self.TempOpen/CloseSound` _returnvalue))

(event `self.ReceiveTick`
  (params (DeltaSeconds :type "Float (single-precision)")))

(event `self.Box.OnComponentBeginOverlap`
  (params (OverlappedComponent :type "PrimitiveComponent Object Reference") (OtherActor :type "Actor Object Reference") (OtherComp :type "PrimitiveComponent Object Reference") (OtherBodyIndex :type Integer) (bFromSweep :type Boolean) (SweepResult :type "HitResult Structure (by ref)"))
  (`self.Action` :!label _label))

(event `self.Box.OnComponentEndOverlap`
  (params (OverlappedComponent :type "PrimitiveComponent Object Reference") (OtherActor :type "Actor Object Reference") (OtherComp :type "PrimitiveComponent Object Reference") (OtherBodyIndex :type Integer))
  (goto _label :!via `Out`))

(event `ActionOn`
  (set `/Game/TPSProPack/Controllers/CharBlueprints/BP_VystudioCharacterController.CanWePickup` true (`self.VSRef`))
  (`self.On/Off Visibility Custom Depth` true)
  (set `self.Timer` 0.1)
  (`KismetSystemLibrary.RetriggerableDelay` (`self.Timer`))
  (set `/Game/TPSProPack/Controllers/CharBlueprints/BP_VystudioCharacterController.CanWePickup` false (`self.VSRef`))
  (`self.ActionOff`))

(event `ActionOff`
  (`self.On/Off Visibility Custom Depth` false))

(event `Open`
  (bind _tempopen_closesound (`self.TempOpen/CloseSound`))
  (switch `/Game/TPSProPack/Controllers/BPObjects/Doors/CloseDoorWithKey/DoorWithKeyCategory` (`self.DoorCategory`)
    (:`NewEnumerator0`
      ;[1 1 1] Door with key
      (if (or (`self.OpenDoor`) (not (`self.DoorClose`)))
        (`AudioComponent.Stop` (`self.TempOpen/CloseSound`) :!label _label_2)
        (if (`self.DoorClose`)
          (set `self.DoorClose` false)
          (`AudioComponent.Play` _tempopen_closesound 0.0)
          (bind (_direction _opendoor) (`Timeline|Timeline_0` :!label _label_3)
            (:`Update`
              (`SceneComponent.K2_SetRelativeRotation` (`self.DoorPlane`) (`KismetMathLibrary.MakeRotator` 0.0 0.0 _opendoor) false false))
            (:`Finished`
              (`AudioComponent.Stop` (`self.TempOpen/CloseSound`))))
          (else
            (set `self.DoorClose` true)
            (`AudioComponent.Play` _tempopen_closesound 0.0)
            (goto _label_3 :!via `Reverse`)))
        (elif (`KismetArrayLibrary.Array_Contains` (`.AllItemsClass_20_540E31F4492AFE481071AABAD10270D5` (break `/Game/TPSProPack/Controllers/CharBlueprints/Structure/BP_ItemStructure` (`/Game/TPSProPack/Controllers/CharBlueprints/BP_VystudioCharacterController.ItemArray` (`self.VSRef`)))) (`self.Key`))
          (`/Engine/EditorBlueprintResources/StandardMacros.DoOnce` false
            (:`Completed`
              (`GameplayStatics.PlaySound2D` (`self.OpenDoorWithKeySound`) 1.0 1.0 0.0 null null)
              (`KismetSystemLibrary.RetriggerableDelay` 2.0)
              (set `self.OpenDoor` true)))
          (else
            (`|ExecutionSequence`
              (:`then_0`
                (`/Engine/EditorBlueprintResources/StandardMacros.DoOnce` false
                  (:`Completed`
                    (bind _returnvalue (`|CreateWidget` "/Game/TPSProPack/Controllers/Interface/UI/BP_FindKeyUI.BP_FindKeyUI_C"))
                    (set `self.FindKeyUI` _returnvalue))))
              (:`then_1`
                (`GameplayStatics.PlaySound2D` (`self.ClosedDoorSound`) 1.0 1.0 0.0 null null)
                (`/Engine/EditorBlueprintResources/StandardMacros.DoOnce` false :!label _label_4
                  (:`Completed`
                    (`UserWidget.AddToViewport` (`self.FindKeyUI`) 0)
                    (`KismetSystemLibrary.RetriggerableDelay` 2.0)
                    (`Widget.RemoveFromParent` (`self.FindKeyUI`))
                    (goto _label_4 :!via `Reset`)))))))))
    (:`NewEnumerator1`
      ;[1 1 1] Door with card detector
      (bind _outactors (`GameplayStatics.GetAllActorsOfClass` (`self.CardDetectors`)))
      (if (or (`/Game/TPSProPack/Controllers/BPObjects/CardDetectors/BP_MasterCardDetectors.OpenStatus` (`|GetArrayItem` _outactors)) (not (`self.DoorClose`)) (`/Game/TPSProPack/Controllers/BPObjects/CardDetectors/BP_MasterCardDetectors.OpenStatus` (`|GetArrayItem` _outactors 1)))
        (set `self.OpenDoor` true)
        (goto _label_2)
        (else
          (`GameplayStatics.PlaySound2D` (`self.ClosedDoorSound`) 1.0 1.0 0.0 null null))))
    (:`NewEnumerator2`
      ;[1 1 1] Door with card detector
      (bind _outactors_2 (`GameplayStatics.GetAllActorsOfClass` (`self.CodeDetector`)))
      (if (or (`/Game/TPSProPack/Controllers/BPObjects/CodeDetectors/BP_MasterCodeDetector.Open` (`|GetArrayItem` _outactors_2)) (not (`self.DoorClose`)))
        (set `self.OpenDoor` true)
        (goto _label_2)
        (else
          (`GameplayStatics.PlaySound2D` (`self.ClosedDoorSound`) 1.0 1.0 0.0 null null))))))

(fn `On/Off Visibility Custom Depth`
  (params (bValue :type Boolean))
  (`PrimitiveComponent.SetRenderCustomDepth` (`self.DoorPlane`) bValue))

(fn `UserConstructionScript`)