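; BP_Master_AutoDoor is an automatic sliding double door, apparently a master Blueprint, that opens when something enters its Box trigger.
; Begin overlap clears DoorClose and plays two timelines that slide Door1 and Door2 along their relative Y axis.
; End overlap waits on a retriggerable delay, then sets DoorClose and reverses both timelines to close the doors.
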(event `self.Box.OnComponentBeginOverlap`
  (params (OverlappedComponent :type "PrimitiveComponent Object Reference") (OtherActor :type "Actor Object Reference") (OtherComp :type "PrimitiveComponent Object Reference") (OtherBodyIndex :type Integer) (bFromSweep :type Boolean) (SweepResult :type "HitResult Structure (by ref)"))
  (set `self.DoorClose` false)
  (`|ExecutionSequence`
    (:`then_0`
      (bind (_direction _open_close_anim) (`Timeline|Open/Close` :!label _label)
        (:`Update`
          (`SceneComponent.K2_SetRelativeLocation` (`self.Door1`) (`KismetMathLibrary.MakeVector` 0.0 _open_close_anim) false false))))
    (:`then_1`
      (bind (_direction_2 _open_close_anim_2) (`Timeline|Timeline_0` :!label _label_2)
        (:`Update`
          (`SceneComponent.K2_SetRelativeLocation` (`self.Door2`) (`KismetMathLibrary.MakeVector` 0.0 _open_close_anim_2) false false))))))

(event `self.Box.OnComponentEndOverlap`
  (params (OverlappedComponent :type "PrimitiveComponent Object Reference") (OtherActor :type "Actor Object Reference") (OtherComp :type "PrimitiveComponent Object Reference") (OtherBodyIndex :type Integer))
  (`KismetSystemLibrary.RetriggerableDelay` 1.0)
  (set `self.DoorClose` true)
  (`|ExecutionSequence`
    (:`then_0`
      (goto _label :!via `Reverse`))
    (:`then_1`
      (goto _label_2 :!via `Reverse`))))

(fn `UserConstructionScript`)