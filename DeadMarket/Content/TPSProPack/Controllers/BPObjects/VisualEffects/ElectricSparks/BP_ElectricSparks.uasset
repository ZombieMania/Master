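; BP_ElectricSparks is a destructible electric lamp effect with three lights, looping or staggered audio and a spark particle system.
; Tick randomly flickers PointLight2 through a DoOnce and retriggerable delay until the Off flag is set.
; Hitting each destructible kills its paired light and sound.
; Overlapping the box drops the main destructible, briefly fires particles, plays break sounds, and shuts down all lights, audio and the trigger.
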(event `self.ReceiveBeginPlay`
  (`AudioComponent.Play` (`self.Audio`) 0.0)
  (`AudioComponent.Play` (`self.Audio1`) 1.0)
  (`AudioComponent.Play` (`self.Audio2`) 2.0))

(event `self.ReceiveTick`
  (params (DeltaSeconds :type "Float (single-precision)"))
  (bind _pointlight2 (`self.PointLight2`))
  (if (not (`self.Off`))
    (`/Engine/EditorBlueprintResources/StandardMacros.DoOnce` false :!label _label
      (:`Completed`
        (`SceneComponent.SetVisibility` _pointlight2 true false)
        (`KismetSystemLibrary.RetriggerableDelay` (`KismetMathLibrary.RandomFloat`))
        (`SceneComponent.SetVisibility` _pointlight2 false false)
        (goto _label :!via `Reset`)))))

(event `self.Box.OnComponentBeginOverlap`
  (params (OverlappedComponent :type "PrimitiveComponent Object Reference") (OtherActor :type "Actor Object Reference") (OtherComp :type "PrimitiveComponent Object Reference") (OtherBodyIndex :type Integer) (bFromSweep :type Boolean) (SweepResult :type "HitResult Structure (by ref)"))
  (bind _particlesystem (`self.ParticleSystem`))
  (`GameplayStatics.PlaySoundAtLocation` "/Game/TPSProPack/Audio/LevelSound/DestroyLampElectro.DestroyLampElectro" (`SceneComponent.K2_GetComponentLocation` (`self.Destructible`)) (struct) 1.0 1.0 0.0 null null null null)
  (`ActorComponent.Activate` _particlesystem false)
  (`PrimitiveComponent.SetSimulatePhysics` (`self.Destructible`) true)
  (`SceneComponent.SetVisibility` (`self.PointLight`) false false)
  (`SceneComponent.SetVisibility` (`self.PointLight1`) false false)
  (`SceneComponent.SetVisibility` (`self.PointLight2`) false false)
  (`KismetSystemLibrary.RetriggerableDelay` 0.5)
  (`ActorComponent.Deactivate` _particlesystem)
  (`PrimitiveComponent.SetCollisionEnabled` (`self.Box`) "NoCollision")
  (`GameplayStatics.PlaySound2D` "/Game/TPSProPack/Audio/LevelSound/DestroyLampSound.DestroyLampSound" 1.0 1.0 0.0 null null)
  (set `self.Off` true)
  (`AudioComponent.Stop` (`self.Audio`))
  (`AudioComponent.Stop` (`self.Audio1`))
  (`AudioComponent.Stop` (`self.Audio2`)))

(event `self.Destructible2.OnComponentHit`
  (params (HitComponent :type "PrimitiveComponent Object Reference") (OtherActor :type "Actor Object Reference") (OtherComp :type "PrimitiveComponent Object Reference") (NormalImpulse :type "Vector Structure") (Hit :type "HitResult Structure (by ref)"))
  (`SceneComponent.SetVisibility` (`self.PointLight1`) false false)
  (`AudioComponent.Stop` (`self.Audio1`)))

(event `self.Destructible1.OnComponentHit`
  (params (HitComponent :type "PrimitiveComponent Object Reference") (OtherActor :type "Actor Object Reference") (OtherComp :type "PrimitiveComponent Object Reference") (NormalImpulse :type "Vector Structure") (Hit :type "HitResult Structure (by ref)"))
  (`SceneComponent.SetVisibility` (`self.PointLight2`) false false)
  (set `self.Off` true)
  (`AudioComponent.Stop` (`self.Audio2`)))

(event `self.Destructible.OnComponentHit`
  (params (HitComponent :type "PrimitiveComponent Object Reference") (OtherActor :type "Actor Object Reference") (OtherComp :type "PrimitiveComponent Object Reference") (NormalImpulse :type "Vector Structure") (Hit :type "HitResult Structure (by ref)"))
  (`SceneComponent.SetVisibility` (`self.PointLight`) false false)
  (`AudioComponent.Stop` (`self.Audio`)))

(fn `UserConstructionScript`)