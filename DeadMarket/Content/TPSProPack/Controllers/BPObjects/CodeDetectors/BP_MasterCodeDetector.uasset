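; Base code-lock actor that opens a keypad widget and checks the entered code against its password.
; Box overlaps adjust the character's TimerOverlap counter, while ActionOn briefly enables pickup and a custom-depth highlight.
; PressCode shows the UI, and Tick polls the widget's flags to run the check or close it.
; A match sets Open once, swaps closed/opened indicators and closes the keypad; a mismatch fires the widget's error event.
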(event `self.ReceiveBeginPlay`
  (bind _asbp_vystudio_character_controller (cast `/Game/TPSProPack/Controllers/CharBlueprints/BP_VystudioCharacterController` (`GameplayStatics.GetPlayerCharacter` 0)))
  (set `self.VSRef` _asbp_vystudio_character_controller)
  (bind _returnvalue (`|CreateWidget` "/Game/TPSProPack/Controllers/BPObjects/CodeDetectors/BP_PressCode.BP_PressCode_C"))
  (set `self.PressCodeWidget` _returnvalue)
  (`SceneComponent.SetVisibility` (`self.WidgetClosed`) true false)
  (`SceneComponent.SetVisibility` (`self.WidgetOpened`) false false))

(event `self.ReceiveTick`
  (params (DeltaSeconds :type "Float (single-precision)"))
  (bind _returnvalue (`GameplayStatics.GetPlayerController` 0))
  (`|ExecutionSequence`
    (:`then_0`
      (if (`/Game/TPSProPack/Controllers/BPObjects/CodeDetectors/BP_PressCode.Ok` (`self.PressCodeWidget`))
        (`/Engine/EditorBlueprintResources/StandardMacros.DoOnce` false :!label _label
          (:`Completed`
            (`self.OK`)))
        (else
          (goto _label :!via `Reset`))))
    (:`then_1`
      (if (`/Game/TPSProPack/Controllers/BPObjects/CodeDetectors/BP_PressCode.CloseWidget` (`self.PressCodeWidget`))
        ;[1 1 1] Closed window
        (set `/Game/TPSProPack/Controllers/BPObjects/CodeDetectors/BP_PressCode.CloseWidget` false (`self.PressCodeWidget`))
        (`Widget.RemoveFromParent` (`self.PressCodeWidget`))
        (set `PlayerController.bShowMouseCursor` false _returnvalue)
        (`WidgetBlueprintLibrary.SetInputMode_GameOnly` _returnvalue)))))

(event `self.Box.OnComponentBeginOverlap`
  (params (OverlappedComponent :type "PrimitiveComponent Object Reference") (OtherActor :type "Actor Object Reference") (OtherComp :type "PrimitiveComponent Object Reference") (OtherBodyIndex :type Integer) (bFromSweep :type Boolean) (SweepResult :type "HitResult Structure (by ref)"))
  (bind _vsref (`self.VSRef`))
  (set `/Game/TPSProPack/Controllers/CharBlueprints/BP_VystudioCharacterController.TimerOverlap` (+ (`/Game/TPSProPack/Controllers/CharBlueprints/BP_VystudioCharacterController.TimerOverlap` _vsref) 1.0) _vsref))

(event `self.Box.OnComponentEndOverlap`
  (params (OverlappedComponent :type "PrimitiveComponent Object Reference") (OtherActor :type "Actor Object Reference") (OtherComp :type "PrimitiveComponent Object Reference") (OtherBodyIndex :type Integer))
  (bind _vsref (`self.VSRef`))
  (set `/Game/TPSProPack/Controllers/CharBlueprints/BP_VystudioCharacterController.TimerOverlap` (- (`/Game/TPSProPack/Controllers/CharBlueprints/BP_VystudioCharacterController.TimerOverlap` _vsref) 1.0) _vsref))

(event `ActionOn`
  (set `/Game/TPSProPack/Controllers/CharBlueprints/BP_VystudioCharacterController.CanWePickup` true (`self.VSRef`))
  (`PrimitiveComponent.SetRenderCustomDepth` (`self.StaticMesh`) true)
  (set `self.Timer` 0.1)
  (`KismetSystemLibrary.RetriggerableDelay` (`self.Timer`))
  (set `/Game/TPSProPack/Controllers/CharBlueprints/BP_VystudioCharacterController.CanWePickup` false (`self.VSRef`))
  (`self.ActionOff`))

(event `ActionOff`
  (`PrimitiveComponent.SetRenderCustomDepth` (`self.StaticMesh`) false))

(event `PressCode`
  (bind _returnvalue (`GameplayStatics.GetPlayerController` 0))
  (bind _presscodewidget (`self.PressCodeWidget`))
  ;[1 1 1] Action status
  (`UserWidget.AddToViewport` _presscodewidget 0)
  (set `PlayerController.bShowMouseCursor` true _returnvalue)
  (`WidgetBlueprintLibrary.SetInputMode_UIOnlyEx` _returnvalue _presscodewidget))

(event `OK`
  (bind _presscodewidget (`self.PressCodeWidget`))
  (bind _presscodewidget_2 (`self.PressCodeWidget`))
  ;[1 1 1] Password controller
  (set `/Game/TPSProPack/Controllers/BPObjects/CodeDetectors/BP_PressCode.Ok` false (`self.PressCodeWidget`))
  (set `self.Equal` 0)
  (for _index (range 4)
    (if (`KismetTextLibrary.EqualEqual_TextText` (`|GetArrayItem` (`/Game/TPSProPack/Controllers/BPObjects/CodeDetectors/BP_PressCode.Password` (`self.PressCodeWidget`)) _index) (`|GetArrayItem` (`self.Password`) _index))
      (set `self.Equal` (+ (`self.Equal`) 1))
      (else
        (set `self.Equal` -1))))
  (if (== (`self.Equal`) (`KismetArrayLibrary.Array_Length` (`self.Password`)))
    (`/Engine/EditorBlueprintResources/StandardMacros.DoOnce` false
      (:`Completed`
        (set `self.Open` true)
        (`SceneComponent.SetVisibility` (`self.WidgetClosed`) false false)
        (`SceneComponent.SetVisibility` (`self.WidgetOpened`) true false)
        (set `/Game/TPSProPack/Controllers/BPObjects/CodeDetectors/BP_PressCode.Closed` false _presscodewidget_2)
        (`/Game/TPSProPack/Controllers/BPObjects/CodeDetectors/BP_PressCode.Opened` _presscodewidget_2)
        (`KismetSystemLibrary.RetriggerableDelay` 0.3)
        (set `/Game/TPSProPack/Controllers/BPObjects/CodeDetectors/BP_PressCode.CloseWidget` true (`self.PressCodeWidget`))))
    (else
      (set `/Game/TPSProPack/Controllers/BPObjects/CodeDetectors/BP_PressCode.Closed` true (`self.PressCodeWidget`))
      (set `self.Open` false)
      (set `/Game/TPSProPack/Controllers/BPObjects/CodeDetectors/BP_PressCode.Error` true _presscodewidget)
      (`/Game/TPSProPack/Controllers/BPObjects/CodeDetectors/BP_PressCode.ErrorEvent` _presscodewidget))))

(fn `UserConstructionScript`)