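; Base interactable locker whose door toggles open and closed through a timeline-driven yaw rotation, with a 2D open/close sound.
; Box overlaps increment or decrement TimerOverlap on the player's BP_VystudioCharacterController, which is cached on BeginPlay.
; ActionOn enables the character's CanWePickup and the door's custom depth highlight, using a short retriggerable delay to clear both once calls stop.
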(event `self.ReceiveBeginPlay`
  (bind _asbp_vystudio_character_controller (cast `/Game/TPSProPack/Controllers/CharBlueprints/BP_VystudioCharacterController` (`GameplayStatics.GetPlayerCharacter` 0)))
  (set `self.VSRef` _asbp_vystudio_character_controller)
  (bind _returnvalue (`GameplayStatics.CreateSound2D` (`self.Open/CloseDoorSound`) 1.0 1.0 1.0 null false false))
  (set `self.TempOpen/CloseSound` _returnvalue))

(event `ActionOn`
  (set `/Game/TPSProPack/Controllers/CharBlueprints/BP_VystudioCharacterController.CanWePickup` true (`self.VSRef`))
  (`self.On/Off Visibility Custom Depth` true)
  (set `self.Timer` 0.1)
  (`KismetSystemLibrary.RetriggerableDelay` (`self.Timer`))
  (set `/Game/TPSProPack/Controllers/CharBlueprints/BP_VystudioCharacterController.CanWePickup` false (`self.VSRef`))
  (`self.ActionOff`))

(event `ActionOff`
  (`self.On/Off Visibility Custom Depth` false))

(event `self.Box.OnComponentBeginOverlap`
  (params (OverlappedComponent :type "PrimitiveComponent Object Reference") (OtherActor :type "Actor Object Reference") (OtherComp :type "PrimitiveComponent Object Reference") (OtherBodyIndex :type Integer) (bFromSweep :type Boolean) (SweepResult :type "HitResult Structure (by ref)"))
  (`self.Action` :!label _label))

(event `self.Box.OnComponentEndOverlap`
  (params (OverlappedComponent :type "PrimitiveComponent Object Reference") (OtherActor :type "Actor Object Reference") (OtherComp :type "PrimitiveComponent Object Reference") (OtherBodyIndex :type Integer))
  (goto _label :!via `Out`))

(event `OpenDoor`
  (bind _tempopen_closesound (`self.TempOpen/CloseSound`))
  (`AudioComponent.Stop` (`self.TempOpen/CloseSound`))
  (if (`self.DoorClose`)
    (set `self.DoorClose` false)
    (`AudioComponent.Play` _tempopen_closesound 0.0)
    (bind (_direction _opendoor) (`Timeline|Open/CloseAnim` :!label _label_2)
      (:`Update`
        (`SceneComponent.K2_SetRelativeRotation` (`self.Door`) (`KismetMathLibrary.MakeRotator` 0.0 0.0 _opendoor) false false))
      (:`Finished`
        (`AudioComponent.Stop` (`self.TempOpen/CloseSound`))))
    (else
      (set `self.DoorClose` true)
      (`AudioComponent.Play` _tempopen_closesound 0.0)
      (goto _label_2 :!via `Reverse`))))

(fn `On/Off Visibility Custom Depth`
  (params (bValue :type Boolean))
  (`PrimitiveComponent.SetRenderCustomDepth` (`self.Door`) bValue))

(fn `UserConstructionScript`)