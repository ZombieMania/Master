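; Master nightstand Blueprint with two racks that the player can open and close independently.
; ActionOn highlights the targeted rack via custom depth and sets the character's CanWePickup, clearing both after a short retriggerable delay.
; Open toggles the hit rack, sliding it along X with its own reversible timeline and 2D sound.
; Two box triggers increment and decrement the character's TimerOverlap counter on overlap begin and end.
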(event `self.ReceiveBeginPlay`
  (bind _asbp_vystudio_character_controller (cast `/Game/TPSProPack/Controllers/CharBlueprints/BP_VystudioCharacterController` (`GameplayStatics.GetPlayerCharacter` 0)))
  (set `self.VSRef` _asbp_vystudio_character_controller)
  (bind _returnvalue (`GameplayStatics.CreateSound2D` (`self.Open/CloseRackSound`) 1.0 1.0 0.0 null false false))
  (set `self.TempOpen/CloseRack1Sound` _returnvalue)
  (bind _returnvalue_2 (`GameplayStatics.CreateSound2D` (`self.Open/CloseRackSound`) 1.0 1.0 0.0 null false false))
  (set `self.TempOpen/CloseRack2Sound` _returnvalue_2))

(event `ActionOn`
  (params (NewParam :type "ActorComponent Object Reference"))
  (bind _rack1 (`self.Rack1`))
  (bind _rack2 (`self.Rack2`))
  (if (== NewParam _rack2)
    (set `/Game/TPSProPack/Controllers/CharBlueprints/BP_VystudioCharacterController.CanWePickup` true (`self.VSRef`))
    (`PrimitiveComponent.SetRenderCustomDepth` _rack2 true)
    (set `self.Timer` 0.1)
    (`KismetSystemLibrary.RetriggerableDelay` (`self.Timer`))
    (set `/Game/TPSProPack/Controllers/CharBlueprints/BP_VystudioCharacterController.CanWePickup` false (`self.VSRef`))
    (`PrimitiveComponent.SetRenderCustomDepth` (`self.Rack2`) false)
    (elif (== NewParam _rack1)
      (set `/Game/TPSProPack/Controllers/CharBlueprints/BP_VystudioCharacterController.CanWePickup` true (`self.VSRef`))
      (`PrimitiveComponent.SetRenderCustomDepth` _rack1 true)
      (set `self.Timer` 0.1)
      (`KismetSystemLibrary.RetriggerableDelay` (`self.Timer`))
      (set `/Game/TPSProPack/Controllers/CharBlueprints/BP_VystudioCharacterController.CanWePickup` false (`self.VSRef`))
      (`PrimitiveComponent.SetRenderCustomDepth` (`self.Rack1`) false))))

(event `self.Box.OnComponentBeginOverlap`
  (params (OverlappedComponent :type "PrimitiveComponent Object Reference") (OtherActor :type "Actor Object Reference") (OtherComp :type "PrimitiveComponent Object Reference") (OtherBodyIndex :type Integer) (bFromSweep :type Boolean) (SweepResult :type "HitResult Structure (by ref)"))
  (set `/Game/TPSProPack/Controllers/CharBlueprints/BP_VystudioCharacterController.TimerOverlap` (+ (`/Game/TPSProPack/Controllers/CharBlueprints/BP_VystudioCharacterController.TimerOverlap` (`self.VSRef`)) 1.0) (`self.VSRef`) :!label _label))

(event `self.Box1.OnComponentBeginOverlap`
  (params (OverlappedComponent :type "PrimitiveComponent Object Reference") (OtherActor :type "Actor Object Reference") (OtherComp :type "PrimitiveComponent Object Reference") (OtherBodyIndex :type Integer) (bFromSweep :type Boolean) (SweepResult :type "HitResult Structure (by ref)"))
  (goto _label))

(event `self.Box1.OnComponentEndOverlap`
  (params (OverlappedComponent :type "PrimitiveComponent Object Reference") (OtherActor :type "Actor Object Reference") (OtherComp :type "PrimitiveComponent Object Reference") (OtherBodyIndex :type Integer))
  (set `/Game/TPSProPack/Controllers/CharBlueprints/BP_VystudioCharacterController.TimerOverlap` (- (`/Game/TPSProPack/Controllers/CharBlueprints/BP_VystudioCharacterController.TimerOverlap` (`self.VSRef`)) 1.0) (`self.VSRef`) :!label _label_2))

(event `self.Box.OnComponentEndOverlap`
  (params (OverlappedComponent :type "PrimitiveComponent Object Reference") (OtherActor :type "Actor Object Reference") (OtherComp :type "PrimitiveComponent Object Reference") (OtherBodyIndex :type Integer))
  (goto _label_2))

(event `Open`
  (params (`Component hit` :type "ActorComponent Object Reference"))
  (bind _tempopen_closerack2sound (`self.TempOpen/CloseRack2Sound`))
  (bind _tempopen_closerack1sound (`self.TempOpen/CloseRack1Sound`))
  (bind (_relativelocation_x _relativelocation_y _relativelocation_z) (`KismetMathLibrary.BreakVector` (`SceneComponent.RelativeLocation` (`self.Rack2`))))
  (bind (_relativelocation_x_2 _relativelocation_y_2 _relativelocation_z_2) (`KismetMathLibrary.BreakVector` (`SceneComponent.RelativeLocation` (`self.Rack1`))))
  (if (== `Component hit` (`self.Rack1`))
    (`AudioComponent.Stop` (`self.TempOpen/CloseRack1Sound`))
    (if (`self.Rack1Closed`)
      (set `self.Rack1Closed` false)
      (`AudioComponent.Play` _tempopen_closerack1sound 0.0)
      (bind (_direction _opendoor) (`Timeline|Open/CloseAnim` :!label _label_3)
        (:`Update`
          (`SceneComponent.K2_SetRelativeLocation` (`self.Rack1`) (`KismetMathLibrary.MakeVector` _opendoor _relativelocation_y_2 _relativelocation_z_2) false false))
        (:`Finished`
          (`AudioComponent.Stop` (`self.TempOpen/CloseRack1Sound`))))
      (else
        (set `self.Rack1Closed` true)
        (`AudioComponent.Play` _tempopen_closerack1sound 0.0)
        (goto _label_3 :!via `Reverse`)))
    (elif (== `Component hit` (`self.Rack2`))
      (`AudioComponent.Stop` (`self.TempOpen/CloseRack2Sound`))
      (if (`self.Rack2Closed`)
        (set `self.Rack2Closed` false)
        (`AudioComponent.Play` _tempopen_closerack2sound 0.0)
        (bind (_direction_2 _opendoor_2) (`Timeline|Timeline_0` :!label _label_4)
          (:`Update`
            (`SceneComponent.K2_SetRelativeLocation` (`self.Rack2`) (`KismetMathLibrary.MakeVector` _opendoor_2 _relativelocation_y _relativelocation_z) false false))
          (:`Finished`
            (`AudioComponent.Stop` (`self.TempOpen/CloseRack2Sound`))))
        (else
          (set `self.Rack2Closed` true)
          (`AudioComponent.Play` _tempopen_closerack2sound 0.0)
          (goto _label_4 :!via `Reverse`))))))

(fn `UserConstructionScript`)