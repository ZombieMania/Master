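; BP_Dummy is a dummy actor from the TPS Pro Pack that reacts once to being overlapped.
; An overlap on either Box or Box1 destroys both components, so neither can fire again.
; Only the Box overlap also shows the Widget, then hides it after a short retriggerable delay; Box1 destroys the boxes without displaying it.
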(event `self.Box.OnComponentBeginOverlap`
  (params (OverlappedComponent :type "PrimitiveComponent Object Reference") (OtherActor :type "Actor Object Reference") (OtherComp :type "PrimitiveComponent Object Reference") (OtherBodyIndex :type Integer) (bFromSweep :type Boolean) (SweepResult :type "HitResult Structure (by ref)"))
  (bind _widget (`self.Widget`))
  (`ActorComponent.K2_DestroyComponent` (`self.Box`))
  (`ActorComponent.K2_DestroyComponent` (`self.Box1`))
  (`SceneComponent.SetVisibility` _widget true false)
  (`KismetSystemLibrary.RetriggerableDelay` 2.0)
  (`SceneComponent.SetVisibility` _widget false false))

(event `self.Box1.OnComponentBeginOverlap`
  (params (OverlappedComponent :type "PrimitiveComponent Object Reference") (OtherActor :type "Actor Object Reference") (OtherComp :type "PrimitiveComponent Object Reference") (OtherBodyIndex :type Integer) (bFromSweep :type Boolean) (SweepResult :type "HitResult Structure (by ref)"))
  (`ActorComponent.K2_DestroyComponent` (`self.Box`))
  (`ActorComponent.K2_DestroyComponent` (`self.Box1`)))

(fn `UserConstructionScript`)