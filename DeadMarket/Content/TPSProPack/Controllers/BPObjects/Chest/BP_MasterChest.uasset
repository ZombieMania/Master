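; Base chest actor for the TPS Pro Pack that the player can highlight and toggle open or closed.
; Box overlaps raise and lower the cached player character's TimerOverlap count.
; ActionOn enables custom depth on the lid and CanWePickup on the character, clearing both after a short retriggerable delay unless called again.
; Open flips DoorClose, plays a timeline forward or in reverse to pitch the lid, and restarts the 2D sound.
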(event `self.ReceiveBeginPlay`
  (bind _asbp_vystudio_character_controller (cast `/Game/TPSProPack/Controllers/CharBlueprints/BP_VystudioCharacterController` (`GameplayStatics.GetPlayerCharacter` 0)))
  (set `self.VSRef` _asbp_vystudio_character_controller)
  (bind _returnvalue (`GameplayStatics.CreateSound2D` (`self.Open/CloseDoorSound`) 1.0 1.0 1.0 null false false))
  (set `self.TempOpen/CloseSound` _returnvalue))

(event `self.Box.OnComponentBeginOverlap`
  (params (OverlappedComponent :type "PrimitiveComponent Object Reference") (OtherActor :type "Actor Object Reference") (OtherComp :type "PrimitiveComponent Object Reference") (OtherBodyIndex :type Integer) (bFromSweep :type Boolean) (SweepResult :type "HitResult Structure (by ref)"))
  (bind _vsref (`self.VSRef`))
  (set `/Game/TPSProPack/Controllers/CharBlueprints/BP_VystudioCharacterController.TimerOverlap` (+ (`/Game/TPSProPack/Controllers/CharBlueprints/BP_VystudioCharacterController.TimerOverlap` _vsref) 1.0) _vsref))

(event `self.Box.OnComponentEndOverlap`
  (params (OverlappedComponent :type "PrimitiveComponent Object Reference") (OtherActor :type "Actor Object Reference") (OtherComp :type "PrimitiveComponent Object Reference") (OtherBodyIndex :type Integer))
  (bind _vsref (`self.VSRef`))
  (set `/Game/TPSProPack/Controllers/CharBlueprints/BP_VystudioCharacterController.TimerOverlap` (- (`/Game/TPSProPack/Controllers/CharBlueprints/BP_VystudioCharacterController.TimerOverlap` _vsref) 1.0) _vsref))

(event `ActionOn`
  (set `/Game/TPSProPack/Controllers/CharBlueprints/BP_VystudioCharacterController.CanWePickup` true (`self.VSRef`))
  (`PrimitiveComponent.SetRenderCustomDepth` (`self.Top`) true)
  (set `self.Timer` 0.1)
  (`KismetSystemLibrary.RetriggerableDelay` (`self.Timer`))
  (set `/Game/TPSProPack/Controllers/CharBlueprints/BP_VystudioCharacterController.CanWePickup` false (`self.VSRef`))
  (`self.ActionOff`))

(event `ActionOff`
  (`PrimitiveComponent.SetRenderCustomDepth` (`self.Top`) false))

(event `Open`
  (bind _tempopen_closesound (`self.TempOpen/CloseSound`))
  (`AudioComponent.Stop` (`self.TempOpen/CloseSound`))
  (if (`self.DoorClose`)
    (set `self.DoorClose` false)
    (`AudioComponent.Play` _tempopen_closesound 0.0)
    (bind (_direction _opendoor) (`Timeline|Timeline_0` :!label _label)
      (:`Update`
        (`SceneComponent.K2_SetRelativeRotation` (`self.Top`) (`KismetMathLibrary.MakeRotator` 0.0 _opendoor) false false))
      (:`Finished`
        (`AudioComponent.Stop` (`self.TempOpen/CloseSound`))))
    (else
      (set `self.DoorClose` true)
      (`AudioComponent.Play` _tempopen_closesound 0.0)
      (goto _label :!via `Reverse`))))

(fn `UserConstructionScript`)