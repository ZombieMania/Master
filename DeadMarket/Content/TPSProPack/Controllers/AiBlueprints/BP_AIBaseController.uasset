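; AI controller for BP_AIMaster_BP enemies that patrols waypoints, hunts the player and shoots.
; Patrol steps forward through waypoints, then jumps back to the first.
; A looping CheckEnemy timer copies the pawn's detection flag to start the hunt, resumes patrol on player death and stops on AI death.
; Firing is a Gate loop with randomized delays, using a line trace for BP_TakeDamage hits and spawning muzzle projectiles toward the impact.
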(event `self.ReceiveBeginPlay`
  ;[1 1 1] Begin play
  (bind _asbp_aimaster_bp (cast `/Game/TPSProPack/Controllers/AiBlueprints/BP_AIMaster_BP` (`self.K2_GetPawn`)))
  (set `self.AIBaseRef` _asbp_aimaster_bp)
  (set `self.WayPoints` (`/Game/TPSProPack/Controllers/AiBlueprints/BP_AIMaster_BP.WayPoint` _asbp_aimaster_bp))
  (bind _returnvalue (`KismetSystemLibrary.K2_SetTimer` null "CheckEnemy" 0.3 true))
  (set `self.CleanTimer` _returnvalue)
  (`|AIMoveTo` _asbp_aimaster_bp (0.0 0.0 0.0) (`|GetArrayItem` (`self.WayPoints`) (`self.CurrentWayPoint`))
    (:`OnSuccess`
      (`KismetSystemLibrary.Delay` 3.0)
      (`self.Patroling`))))

(event `Patroling`
  ;[1 1 1] Patroling
  (if (not (`self.FoundEnemy`))
    (if (`self.WalkBack`)
      (set `self.CurrentWayPoint` (* (`self.CurrentWayPoint`) 0))
      (`|AIMoveTo` null (0.0 0.0 0.0) (`|GetArrayItem` (`self.WayPoints`) (`self.CurrentWayPoint`))
        (:`OnSuccess`
          (if (<= (`self.CurrentWayPoint`) 0)
            (set `self.WalkBack` false))))
      (else
        (set `self.CurrentWayPoint` (+ (`self.CurrentWayPoint`) 1))
        (`|AIMoveTo` null (0.0 0.0 0.0) (`|GetArrayItem` (`self.WayPoints`) (`self.CurrentWayPoint`))
          (:`OnSuccess`
            (if (>= (`self.CurrentWayPoint`) (- (`KismetArrayLibrary.Array_Length` (`self.WayPoints`)) 1))
              (set `self.WalkBack` true))))))
    (`KismetSystemLibrary.Delay` 0.2)
    (`self.Patroling`)))

(event `CheckEnemy`
  (bind _aibaseref (`self.AIBaseRef`))
  ;[1 1 1] Check enemy
  (if (`/Game/TPSProPack/Controllers/CharBlueprints/BP_VystudioCharacterController.IsDeath?` (cast `/Game/TPSProPack/Controllers/CharBlueprints/BP_VystudioCharacterController` (`GameplayStatics.GetPlayerCharacter` 0) :!pure true))
    (if (`/Game/TPSProPack/Controllers/AiBlueprints/BP_AIMaster_BP.EquipWeapon` (`self.AIBaseRef`))
      (set `self.FoundEnemy` false)
      (`KismetSystemLibrary.Delay` 1.0)
      (`/Engine/EditorBlueprintResources/StandardMacros.DoOnce` false
        (:`Completed`
          (`self.StopFire`)
          (`/Game/TPSProPack/Controllers/AiBlueprints/BP_AIMaster_BP.EnableCombat` (`self.AIBaseRef`))
          (`KismetSystemLibrary.Delay` 2.0)
          (set `self.CurrentWayPoint` 0)
          (`self.Patroling`))))
    (elif (`/Game/TPSProPack/Controllers/AiBlueprints/BP_AIMaster_BP.IsDeath?` _aibaseref)
      (`KismetSystemLibrary.K2_ClearAndInvalidateTimerHandle` (`self.CleanTimer`))
      (`self.StopMovement`)
      (else
        (bind _output_get (set `self.FoundEnemy` (`/Game/TPSProPack/Controllers/AiBlueprints/BP_AIMaster_BP.EnemyFound` _aibaseref)))
        (if _output_get
          (`|ExecutionSequence`
            (:`then_0`
              (`KismetSystemLibrary.Delay` 0.5)
              (`/Game/TPSProPack/Controllers/AiBlueprints/BP_AIMaster_BP.ScanEnemy` (`self.AIBaseRef`))
              (`self.OnHunt`))
            (:`then_1`
              (`/Engine/EditorBlueprintResources/StandardMacros.DoOnce` false
                (:`Completed`
                  (`/Game/TPSProPack/Controllers/AiBlueprints/BP_AIMaster_BP.EnableCombat` (`self.AIBaseRef`)))))))))))

(event `OnHunt`
  ;[1 1 1] Hunt
  (`|AIMoveTo` null (0.0 0.0 0.0) (`GameplayStatics.GetPlayerCharacter` 0) (`self.Radius`)
    (:`OnSuccess`
      _)
    (:`OnFail`
      _))
  (if (`/Game/TPSProPack/Controllers/AiBlueprints/BP_AIMaster_BP.Active` (`self.AIBaseRef`))
    (`self.Fire`)
    (set `self.Radius` 3000.0)
    (else
      (`self.StopFire`)
      (set `self.Radius` 1000.0)
      (`KismetSystemLibrary.Delay` 10.0)
      (set `/Game/TPSProPack/Controllers/AiBlueprints/BP_AIMaster_BP.Active` false (`self.AIBaseRef`)))))

(event `Fire`
  (bind _asbp_vystudio_character_controller (cast `/Game/TPSProPack/Controllers/CharBlueprints/BP_VystudioCharacterController` (`GameplayStatics.GetPlayerCharacter` 0) :!pure true))
  (bind _visiondirectionarrow (`/Game/TPSProPack/Controllers/AiBlueprints/BP_AIMaster_BP.VisionDirectionArrow` (`self.AIBaseRef`)))
  (bind _returnvalue (`SceneComponent.K2_GetComponentLocation` _visiondirectionarrow))
  (bind _returnvalue_2 (`SceneComponent.GetSocketLocation` (`/Game/TPSProPack/Controllers/WeaponBP/Weapons/BP_Weapon.SkeletalMesh` (`/Game/TPSProPack/Controllers/AiBlueprints/BP_AIMaster_BP.WeaponBP` (`self.AIBaseRef`))) "MuzzleFlash"))
  ;[1 1 1] Fire
  (`|ExecutionSequence`
    (:`then_0`
      (goto _label :!via `Open`))
    (:`then_1`
      (`/Engine/EditorBlueprintResources/StandardMacros.Gate` true :!label _label
        (:`Exit`
          (`|ExecutionSequence`
            (:`then_0`
              (`KismetSystemLibrary.RetriggerableDelay` (`KismetMathLibrary.RandomFloatInRange` (`KismetMathLibrary.RandomFloatInRange` 0.1 0.2) (`KismetMathLibrary.RandomFloatInRange` 0.65 1.0)))
              (if (or (`/Game/TPSProPack/Controllers/AiBlueprints/BP_AIMaster_BP.IsDeath?` (`self.AIBaseRef`)) (`/Game/TPSProPack/Controllers/CharBlueprints/BP_VystudioCharacterController.IsDeath?` _asbp_vystudio_character_controller))
                (`self.StopFire` :!label _label_2)
                (else
                  (goto _label))))
            (:`then_1`
              (if (`/Game/TPSProPack/Controllers/CharBlueprints/BP_VystudioCharacterController.IsDeath?` _asbp_vystudio_character_controller)
                (goto _label_2)
                (else
                  (bind (_outhit _returnvalue_3) (`KismetSystemLibrary.LineTraceSingle` _returnvalue (+ _returnvalue (* (`SceneComponent.GetForwardVector` _visiondirectionarrow) 10000.0)) "TraceTypeQuery2" false (`|MakeArray` (`self.AIBaseRef`) :!type "Actor Object Reference")))
                  (if _returnvalue_3
                    _
                    (else
                      _))
                  (`GameplayStatics.PlaySound2D` "/Game/TPSProPack/Audio/ShootSound/ak74_shoot_Cue.ak74_shoot_Cue" 1.0 1.0 0.0 null null)
                  (bind (_bblockinghit _binitialoverlap _time _distance _location _impactpoint _normal _impactnormal _physmat _hitactor _hitcomponent _hitbonename _bonename _hititem _elementindex _faceindex _tracestart _traceend) (`GameplayStatics.BreakHitResult` _outhit))
                  (if (`KismetSystemLibrary.DoesImplementInterface` _hitactor "/Game/TPSProPack/Controllers/AiBlueprints/BP_TakeDamage.BP_TakeDamage_C")
                    ;;[1 1 1] Damage
                    (message `/Game/TPSProPack/Controllers/AiBlueprints/BP_TakeDamage.iTakeDamage` _hitactor _hitbonename (`KismetMathLibrary.RandomFloatInRange` 20.0 40.0)))
                  (`|SpawnActorFromClass` (`self.ProjectileBP`) (`KismetMathLibrary.MakeTransform` _returnvalue_2 (`KismetMathLibrary.FindLookAtRotation` _returnvalue_2 (`KismetMathLibrary.SelectVector` _impactpoint _traceend _returnvalue_3))) "Undefined" "OverrideRootScale" null null))))))))))

(event `StopFire`
  ;[1 1 1] Fire
  (goto _label :!via `Close`))

(fn `UserConstructionScript`)