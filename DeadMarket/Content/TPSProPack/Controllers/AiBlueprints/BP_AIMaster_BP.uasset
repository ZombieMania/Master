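; Base armed AI enemy character with health, a HUD widget, a spawned weapon and player detection.
; Damage kills instantly on headshots, otherwise briefly shows the widget; death ragdolls the mesh and disables capsule collision.
; Pawn sensing flags living players by sight or sound and plays the equip montage once, resetting on dead players.
; A flip-flop event swaps weapon sockets, and ScanEnemy line-traces forward for damageable actors.
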(event `self.ReceiveBeginPlay`
  ;[1 1 1] Begin play
  (set `self.CurrentHealth` (`self.MaxHealth`))
  (bind _asbp_ai_hud (cast `/Game/TPSProPack/Controllers/AiBlueprints/BP_AI_HUD` (`WidgetComponent.GetUserWidgetObject` (`self.Widget`))))
  (set `/Game/TPSProPack/Controllers/AiBlueprints/BP_AI_HUD.Owner` self _asbp_ai_hud)
  (`self.SpawnDefaultWeapon`)
  (`SceneComponent.SetVisibility` (`self.Widget`) false false))

(event `/Game/TPSProPack/Controllers/AiBlueprints/BP_TakeDamage.iTakeDamage`
  (params (BoneName :type Name) (Damage :type "Float (double-precision)"))
  (bind _currenthealth (`self.CurrentHealth`))
  ;[1 1 1] Damage
  (if (== BoneName "Head")
    (set `self.CurrentHealth` 0.0)
    (else
      (set `self.EnemyFound` true)
      (set `self.CurrentHealth` (- _currenthealth Damage))))
  (if (<= _currenthealth 0.0)
    (set `self.IsDeath?` true)
    (`SkeletalMeshComponent.SetAllBodiesSimulatePhysics` (`self.Mesh`) true)
    (`PrimitiveComponent.SetCollisionEnabled` (`self.CapsuleComponent`) "NoCollision")
    (`SceneComponent.SetVisibility` (`self.Widget`) false false)
    (else
      (set `self.IsDeath?` false)
      (`SceneComponent.SetVisibility` (`self.Widget`) true false)
      (`KismetSystemLibrary.Delay` 2.0)
      (`SceneComponent.SetVisibility` (`self.Widget`) false false))))

(event `SpawnDefaultWeapon`
  ;[1 1 1] Spawn default weapon
  (bind _returnvalue (`|SpawnActorFromClass` (`self.WeaponClass`) (`SceneComponent.K2_GetComponentToWorld` (`self.Sphere`)) "Undefined" "OverrideRootScale" null (struct) null))
  (bind _output_get (set `self.WeaponBP` _returnvalue))
  (`self.K2_AttachToComponent` _output_get (`self.Mesh`) (`self.RifleSocketUnarmed`) "KeepWorld" "KeepWorld" "KeepWorld" true)
  (`PrimitiveComponent.SetSimulatePhysics` (`/Game/TPSProPack/Controllers/WeaponBP/Weapons/BP_Weapon.SkeletalMesh` _output_get) false)
  (`/Game/TPSProPack/Controllers/WeaponBP/Weapons/BP_Weapon.DestroySphere` _returnvalue)
  (if (`self.IsDeath?`)
    (`self.K2_AttachToComponent` _returnvalue null (`self.RifleSocketUnarmed`) "KeepWorld" "KeepWorld" "KeepWorld" true)))

(event `Equip/Unequip`
  ;[1 1 1] Equip/Unequip
  (`/Engine/EditorBlueprintResources/StandardMacros.FlipFlop`
    (:`A`
      (`self.K2_AttachToComponent` (`self.WeaponBP`) (`self.Mesh`) (`self.RifleSocketArmed`) "KeepRelative" "KeepRelative" "KeepRelative" true)
      (set `self.EquipWeapon` true))
    (:`B`
      (`self.K2_AttachToComponent` (`self.WeaponBP`) (`self.Mesh`) (`self.RifleSocketUnarmed`) "KeepRelative" "KeepRelative" "KeepRelative" true)
      (set `self.EquipWeapon` false)
      (set `self.EnemyFound` false))))

(event `EnableCombat`
  ;[1 1 1] Combat event
  (`/Engine/EditorBlueprintResources/StandardMacros.DoOnce` false :!label _label
    (:`Completed`
      (`self.PlayAnimMontage` "/Game/TPSProPack/DemoContent/AnimStarterPack/Equip_Rifle_Standing_Montage_Demo.Equip_Rifle_Standing_Montage_Demo"))))

(event `self.PawnSensing.OnSeePawn`
  (params (Pawn :type "Pawn Object Reference"))
  ;[1 1 1] See
  (bind _asbp_vystudio_character_controller (cast `/Game/TPSProPack/Controllers/CharBlueprints/BP_VystudioCharacterController` Pawn))
  (if (`/Game/TPSProPack/Controllers/CharBlueprints/BP_VystudioCharacterController.IsDeath?` _asbp_vystudio_character_controller)
    (set `self.EnemyFound` false)
    (goto _label :!via `Reset`)
    (else
      (set `self.EnemyFound` true)
      (`self.EnableCombat`))))

(event `self.PawnSensing.OnHearNoise`
  (params (Instigator :type "Pawn Object Reference") (Location :type "Vector Structure (by ref)") (Volume :type "Float (single-precision)"))
  ;[1 1 1] Hear
  (bind _asbp_vystudio_character_controller (cast `/Game/TPSProPack/Controllers/CharBlueprints/BP_VystudioCharacterController` Instigator))
  (if (`/Game/TPSProPack/Controllers/CharBlueprints/BP_VystudioCharacterController.IsDeath?` _asbp_vystudio_character_controller)
    (set `self.EnemyFound` false)
    (goto _label :!via `Reset`)
    (else
      (set `self.EnemyFound` true)
      (`self.EnableCombat`))))

(event `ScanEnemy`
  (bind _visiondirectionarrow (`self.VisionDirectionArrow`))
  (bind _returnvalue (`SceneComponent.K2_GetComponentLocation` _visiondirectionarrow))
  ;[1 1 1] Search player
  (bind (_outhit _returnvalue_2) (`KismetSystemLibrary.LineTraceSingle` _returnvalue (+ _returnvalue (* (`SceneComponent.GetForwardVector` _visiondirectionarrow) 10000.0)) "TraceTypeQuery2" false (`|MakeArray` self (`self.Weapon`) (`self.WeaponBP`) :!type "Actor Object Reference")))
  (if _returnvalue_2
    (bind (_bblockinghit _binitialoverlap _time _distance _location _impactpoint _normal _impactnormal _physmat _hitactor) (`GameplayStatics.BreakHitResult` _outhit))
    (if (`KismetSystemLibrary.DoesImplementInterface` _hitactor "/Game/TPSProPack/Controllers/AiBlueprints/BP_TakeDamage.BP_TakeDamage_C")
      (cast `/Game/TPSProPack/Controllers/CharBlueprints/BP_VystudioAiController` _hitactor
        (:`then`
          (set `self.EnemayLocation` _impactpoint))
        (:`CastFailed`
          (set `self.EnemayLocation` (0.0 0.0 0.0))))
      (set `self.Active` true)
      (else
        (set `self.Active` false)))))

(fn `UserConstructionScript`)