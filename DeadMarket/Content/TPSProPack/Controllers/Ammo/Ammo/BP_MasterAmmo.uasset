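; BP_MasterAmmo is an ammo pickup, apparently the parent of the PM, rifle, SVD and shotgun ammo Blueprints.
; Sphere overlaps adjust the player character's TimerOverlap counter.
; Depthon enables pickup, the widget and custom-depth highlight until a short retriggerable delay lapses.
; PickUpAmmo maps the pickup's class to an ammo type, adds its amount to the matching character counter, and destroys the pickup.
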(event `self.ReceiveBeginPlay`
  ;[1 1 1] BeginPlay
  (bind _asbp_vystudio_character_controller (cast `/Game/TPSProPack/Controllers/CharBlueprints/BP_VystudioCharacterController` (`GameplayStatics.GetPlayerCharacter` 0)))
  (set `self.VSRef` _asbp_vystudio_character_controller))

(event `self.Sphere.OnComponentBeginOverlap`
  (params (OverlappedComponent :type "PrimitiveComponent Object Reference") (OtherActor :type "Actor Object Reference") (OtherComp :type "PrimitiveComponent Object Reference") (OtherBodyIndex :type Integer) (bFromSweep :type Boolean) (SweepResult :type "HitResult Structure (by ref)"))
  ;[1 1 1] Begin/End overlap
  (`self.OverlapTimer` :!label _label))

(event `self.Sphere.OnComponentEndOverlap`
  (params (OverlappedComponent :type "PrimitiveComponent Object Reference") (OtherActor :type "Actor Object Reference") (OtherComp :type "PrimitiveComponent Object Reference") (OtherBodyIndex :type Integer))
  ;[1 1 1] Begin/End overlap
  (goto _label :!via `out`))

(event `Depth on`
  ;[1 1 1] Depth On/Off
  (set `/Game/TPSProPack/Controllers/CharBlueprints/BP_VystudioCharacterController.CanWePickup` true (`self.VSRef`))
  (`SceneComponent.SetVisibility` (`self.Widget`) true true)
  (`PrimitiveComponent.SetRenderCustomDepth` (`self.StaticMesh`) true)
  (bind _output_get (set `self.Timer` 0.1))
  (`KismetSystemLibrary.RetriggerableDelay` _output_get)
  (set `/Game/TPSProPack/Controllers/CharBlueprints/BP_VystudioCharacterController.CanWePickup` false (`self.VSRef`))
  (`self.Depth off`))

(event `Depth off`
  ;[1 1 1] Depth On/Off
  (`SceneComponent.SetVisibility` (`self.Widget`) false true)
  (`PrimitiveComponent.SetRenderCustomDepth` (`self.StaticMesh`) false)
  (set `/Game/TPSProPack/Controllers/CharBlueprints/BP_VystudioCharacterController.CanWePickup` false (`self.VSRef`)))

(event `PickUpAmmo`
  (params (Pickup :type "Actor Object Reference"))
  ;[1 1 1] PickUp
  (bind _output_get (set `self.Pickup` Pickup))
  (bind _returnvalue (`GameplayStatics.GetObjectClass` _output_get))
  (if (== _returnvalue "/Game/TPSProPack/Controllers/Ammo/Ammo/BP_PM_Ammo.BP_PM_Ammo_C")
    (set `self.Ammo` "NewEnumerator1")
    (switch `/Game/TPSProPack/Controllers/Ammo/Ammo/AmmoEnum` (`self.Ammo`) :!label _label_2
      (:`NewEnumerator0`
        (`self.AK74_Ammo`))
      (:`NewEnumerator1`
        (`self.PM_Ammo`))
      (:`NewEnumerator2`
        (`self.SVD_Ammo`))
      (:`NewEnumerator4`
        (`self.Shotgun_Ammo`)))
    (`SceneComponent.SetVisibility` (`self.Sphere`) false false)
    (`SceneComponent.SetVisibility` (`self.Widget`) false false)
    (`SceneComponent.SetVisibility` (`self.StaticMesh`) false false)
    (`self.Depth off`)
    (`self.K2_DestroyActor` (`self.Pickup`))
    (elif (== _returnvalue "/Game/TPSProPack/Controllers/Ammo/Ammo/BP_Rifle_Ammo.BP_Rifle_Ammo_C")
      (set `self.Ammo` "NewEnumerator0")
      (goto _label_2)
      (elif (== _returnvalue "/Game/TPSProPack/Controllers/Ammo/Ammo/BP_SVD_Ammo.BP_SVD_Ammo_C")
        (set `self.Ammo` "NewEnumerator2")
        (goto _label_2)
        (elif (== _returnvalue "/Game/TPSProPack/Controllers/Ammo/Ammo/BP_Shotgun_Ammo.BP_Shotgun_Ammo_C")
          (set `self.Ammo` "NewEnumerator4")
          (goto _label_2))))))

(fn `UserConstructionScript`
  (bind (_ammotype_ammoclass _ammotype_ammotype _ammotype_current) (break `/Game/TPSProPack/Controllers/Ammo/Ammo/AmmoType` (`self.AmmoType`)))
  (set `self.AmmoType` (make `/Game/TPSProPack/Controllers/Ammo/Ammo/AmmoType` (`GameplayStatics.GetObjectClass` self) _ammotype_ammotype _ammotype_current)))